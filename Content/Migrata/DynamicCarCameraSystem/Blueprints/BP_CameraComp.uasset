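; Car camera component that switches between first- and third-person spring-arm views, with mouse look, zoom and held side or rear views.
; Each tick, local velocity and its change sway the first-person arm and shift the third-person rig, which smoothly trails the car's rotation.
; Accumulated forward/backward travel automatically swings the chase view between rear and front.
; Speed-scaled shake affects both views, and mouse look times out after a delay.
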(event `MouseActivating`
  (params (MouseX :type "Float (double-precision)") (MouseY :type "Float (double-precision)") (`MouseActive?` :type Boolean))
  ;[1 0.06025 0] MouseActivating
  (if (not `MouseActive?`)
    (`self.MouseRotating` MouseX MouseY)
    (`KismetSystemLibrary.Delay` 8.0)
    (set `self.MouseRotation?` false)
    (`SceneComponent.K2_SetRelativeRotation` :`self` (`self.SceneComponent1St`))))

(event `ButtonReleased`
  ;[1 0.2821 0] ButtonReleased/SetCameraBAck
  (`self.CameraBackButton`))

(event `self.ReceiveTick`
  (params (DeltaSeconds :type "Float (single-precision)"))
  (bind _returnvalue (`GameplayStatics.GetPlayerCameraManager` 0))
  (bind _mesh (`self.Mesh`))
  (set `self.DeltaSec` DeltaSeconds)
  ;[0 0.07224 1] GetMeshLocalVelocity
  (`|ExecutionSequence`
    (:`then_0`
      (bind _returnvalue_2 (`PrimitiveComponent.GetPhysicsLinearVelocityAtPoint` _mesh (`SceneComponent.K2_GetComponentLocation` _mesh) "None"))
      ;[0 1 0.1339] 3rdCameraLocation
      (switch `int` (`self.CameraID`)
        (:`0`
          (bind _returnvalue_3 (`KismetMathLibrary.TransformDirection` (`KismetMathLibrary.InvertTransform` (`SceneComponent.K2_GetComponentToWorld` _mesh)) _returnvalue_2))
          (bind _z (.z (`KismetMathLibrary.VInterpTo` (`SceneComponent.RelativeLocation` (`self.SpringArm1st`)) (* (/ (/ (- _returnvalue_3 (`self.Prev_Direction`)) (`self.DeltaSec`)) 140.0) -1.0) (`self.DeltaSec`) 2.0)))
          (bind _returnvalue_4 (/ (- (* (.x (`KismetMathLibrary.VInterpTo` (`SceneComponent.RelativeLocation` (`self.SpringArm1st`)) (* (/ (/ (- _returnvalue_3 (`self.Prev_Direction`)) (`self.DeltaSec`)) 140.0) -1.0) (`self.DeltaSec`) 2.0)) 2.0) (/ (`self.CameraMov`) 2.0)) 2.0))
          (bind _returnvalue_5 (`KismetMathLibrary.FClamp` (/ (.y _returnvalue_3) 100.0) -4.0 4.0))
          ;[0 1 0.1196] 1stCameraRotation
          (`SceneComponent.K2_SetRelativeLocation` (`self.SpringArm1st`) (`KismetMathLibrary.MakeVector` _returnvalue_4 _returnvalue_5 _z) false false)
          (set `self.Prev_Direction` _returnvalue_3)
          ;[0 1 0.9734] 1StCameraRotation
          (`SceneComponent.K2_SetRelativeRotation` (`self.SpringArm1st`) (`KismetMathLibrary.MakeRotator` _returnvalue_5 (* (+ (/ _returnvalue_4 2.0) (/ _z 2.0)) -1.0)) false false)
          (`|ExecutionSequence`
            (:`then_0`
              (`self.ProperRotMaker` (`self.SpringArm1st`)))
            (:`then_1`
              (`self.SetYRotation` (`self.SpringArm1st`)))))
        (:`1`
          (`SceneComponent.K2_SetRelativeLocation` (`self.SceneComponent3rd`) (`KismetMathLibrary.MakeVector` (/ (- (* (.x (`KismetMathLibrary.VInterpTo` (`SceneComponent.RelativeLocation` (`self.SceneComponent3rd`)) (* (/ (/ (- _returnvalue_3 (`self.Prev_Direction`)) (`self.DeltaSec`)) 40.0) -1.0) (`self.DeltaSec`) 2.0)) 2.0) (`self.CameraMov`)) 2.0) 0.0 (.z (`KismetMathLibrary.VInterpTo` (`SceneComponent.RelativeLocation` (`self.SceneComponent3rd`)) (* (/ (/ (- _returnvalue_3 (`self.Prev_Direction`)) (`self.DeltaSec`)) 40.0) -1.0) (`self.DeltaSec`) 2.0))) false false)
          (set `self.Prev_Direction` _returnvalue_3)
          ;[1 0.06025 0] UseMouseRotation?
          (if (not (`self.MouseRotation?`))
            ;[0 1 0.9734] 3RdCameraRotation
            (`|ExecutionSequence`
              (:`then_0`
                ;[0 0.9983 1] CarSpeed> CameraRotation on Y<
                (`SceneComponent.K2_AddRelativeRotation` (`self.SpringArm3rd`) (`KismetMathLibrary.MakeRotator` 0.0 (`KismetMathLibrary.FClamp` (/ (.x (`self.Prev_Direction`)) 30000.0) 0.0 0.1)) false false)
                ;[0 1 0.9734] SmoothCarFollowingRotation
                (`SceneComponent.K2_SetRelativeRotation` (`self.SpringArm3rd`) (`KismetMathLibrary.MakeRotator` 0.0 (- (.pitch (`KismetMathLibrary.RInterpTo` (`KismetMathLibrary.MakeRotator` 0.0 (+ (.pitch (`SceneComponent.RelativeRotation` (`self.SpringArm3rd`))) 25.0) (.yaw (`SceneComponent.RelativeRotation` (`self.SpringArm3rd`)))) (`self.Prev_Rotation`) (`self.DeltaSec`) (`self.3rdInterpSpeed`))) 25.0) (.yaw (`KismetMathLibrary.RInterpTo` (`KismetMathLibrary.MakeRotator` 0.0 (+ (.pitch (`SceneComponent.RelativeRotation` (`self.SpringArm3rd`))) 25.0) (.yaw (`SceneComponent.RelativeRotation` (`self.SpringArm3rd`)))) (`self.Prev_Rotation`) (`self.DeltaSec`) (`self.3rdInterpSpeed`)))) false false)
                (set `self.Prev_Rotation` (`SceneComponent.K2_GetComponentRotation` (`self.SceneComponent3rd`))))
              (:`then_1`
                (`self.ProperRotMaker` (`self.SpringArm3rd`)))
              (:`then_2`
                (`self.SetYRotation` (`self.SpringArm3rd`))))))))
    (:`then_1`
      ;[1 1 1] AutomaticCameraBAck
      (`self.CheckCarDistanceTraveled`))
    (:`then_2`
      ;[0.7535 0 1] CameraShakeBasedOnCarSpeed
      (`self.SwitchCameraID`
        (:`FirstCamera`
          (`PlayerCameraManager.StartMatineeCameraShake` :`self` _returnvalue :`ShakeClass` "/Game/Migrata/DynamicCarCameraSystem/Blueprints/BP_CameraShakeBlup.BP_CameraShakeBlup_C" :`Scale` (/ (- (`KismetMathLibrary.FClamp` (`KismetMathLibrary.Abs` (.x (`self.Prev_Direction`))) 700.0 2000.0) 700.0) 5000.0)))
        (:`ThirdCamera`
          (`PlayerCameraManager.StartMatineeCameraShake` :`self` _returnvalue :`ShakeClass` "/Game/Migrata/DynamicCarCameraSystem/Blueprints/BP_CameraShakeBlup.BP_CameraShakeBlup_C" :`Scale` (/ (- (`KismetMathLibrary.FClamp` (`KismetMathLibrary.Abs` (.x (`self.Prev_Direction`))) 700.0 2000.0) 700.0) 475.0)))))))

(fn `ButtonPressed`
  (params (FixedCameraRot3rd :type "Float (double-precision)"))
  (bind _returnvalue (`KismetMathLibrary.MakeRotator` 0.0 0.0 (`self.FixedCameraRot3rd`)))
  ;[1 1 1] If button pressed (For example "E" and "Q") set side view of the car or back view (Middle mouse button)
  (set `self.FixedCameraRot3rd` FixedCameraRot3rd)
  (set `self.3rdInterpSpeed` 10.0)
  (`self.SwitchCameraID`
    (:`FirstCamera`
      (`SceneComponent.K2_SetRelativeRotation` (`self.SceneComponent1St`) (`KismetMathLibrary.NegateRotator` _returnvalue) false false))
    (:`ThirdCamera`
      (`SceneComponent.K2_SetRelativeRotation` (`self.SceneComponent3rd`) _returnvalue false false)
      (set `self.UseRotation?` false))))

(fn `CameraZoom`
  (params (AxisValue :type "Float (double-precision)"))
  ;[1 1 1] Set Spring arm smooth lenght based on mouse wheel Axis value
  (bind _output_get (set `self.ZoomTarget` (`KismetMathLibrary.FClamp` (+ (`self.ZoomTarget`) (* AxisValue (`self.ZoomSensetive`))) 400.0 600.0)))
  (set `SpringArmComponent.TargetArmLength` (`KismetMathLibrary.FInterpTo` (`SpringArmComponent.TargetArmLength` (`self.SpringArm3rd`)) _output_get (`self.DeltaSec`) 5.0) (`self.SpringArm3rd`)))

(fn `ChangeCamera`
  (bind _3rdcamera (`self.3rdcamera`))
  (bind _1stcamera (`self.1stCamera`))
  (`self.SwitchCameraID`
    (:`FirstCamera`
      (`self.SetActive` _1stcamera false false)
      (`self.SetActive` _3rdcamera true false)
      (set `self.CameraID` 1))
    (:`ThirdCamera`
      (`self.SetActive` _3rdcamera false false)
      (`self.SetActive` _1stcamera true false)
      (set `self.CameraID` 0))))

(fn `CheckCarDistanceTraveled`
  (returns (LastRotation :type "Float (double-precision)"))
  (bind _returnvalue (`KismetMathLibrary.FClamp` (/ (`self.CarTransform`) 5.0) -180.0 0.0))
  ;[1 1 1] Check car traveled distance and if distance is more than (Max and Min) smoothly set camera back or front view
  (bind _output_get (set `self.CarTransform` (`KismetMathLibrary.FClamp` (+ (* (.x (`self.Prev_Direction`)) (`self.DeltaSec`)) (`self.CarTransform`)) -1000.0 100.0)))
  (if (`self.UseRotation?`)
    (`SceneComponent.K2_SetRelativeRotation` (`self.SceneComponent3rd`) (`KismetMathLibrary.MakeRotator` 0.0 0.0 _returnvalue) false false)
    (if (`KismetMathLibrary.InRange_FloatFloat` _output_get -1000.0 100.0)
      (set `self.3rdInterpSpeed` (`self.CameraPhasingCpeed`))
      (else
        (set `self.3rdInterpSpeed` 10.0)))
    (return _returnvalue)))

(fn `MouseRotating`
  (params (MouseX :type "Float (double-precision)") (MouseY :type "Float (double-precision)"))
  ;[1 1 1] If mouse is rotating set mouse rotation mode
  (`SceneComponent.K2_SetRelativeRotation` (`self.SpringArm3rd`) (`KismetMathLibrary.MakeRotator` 0.0 (`KismetMathLibrary.FClamp` (+ MouseY (.pitch (`SceneComponent.RelativeRotation` (`self.SpringArm3rd`)))) -55.0 0.0) (`KismetMathLibrary.ClampAxis` (+ MouseX (.yaw (`SceneComponent.RelativeRotation` (`self.SpringArm3rd`)))))) false false)
  (`SceneComponent.K2_SetRelativeRotation` (`self.SceneComponent1St`) (`KismetMathLibrary.MakeRotator` 0.0 (`KismetMathLibrary.FClamp` (+ MouseY (.pitch (`SceneComponent.RelativeRotation` (`self.SpringArm3rd`)))) -55.0 0.0) (`KismetMathLibrary.ClampAxis` (+ MouseX (.yaw (`SceneComponent.RelativeRotation` (`self.SpringArm3rd`)))))) false false)
  (set `self.MouseRotation?` true))

(fn `NearlyEqual`
  (returns (NearlyEqual :type Boolean))
  ;[1 1 1] Check is Spring arm rotation is close to Mesh Rotation
  (return (`KismetMathLibrary.NearlyEqual_FloatFloat` (.yaw (`SceneComponent.RelativeRotation` (`self.SpringArm3rd`))) (.yaw (`SceneComponent.K2_GetComponentRotation` (`self.Mesh`))) 2.0)))

(fn `ProperRotMaker`
  (params (Target :type "SceneComponent Object Reference"))
  (bind _returnvalue (`KismetMathLibrary.Abs` (.yaw (`KismetMathLibrary.RInterpTo` (`SceneComponent.RelativeRotation` (`self.Mesh`)) (`SceneComponent.RelativeRotation` Target) (`self.DeltaSec`) 2.0))))
  ;[1 1 1] Makes proper rotation on x axis (Based on "Y" velocity)
  (if (> (`self.Y_Velocity`) _returnvalue)
    (set `self.CameraMov` (- (`self.Y_Velocity`) _returnvalue))
    (else
      (set `self.CameraMov` (- _returnvalue (`self.Y_Velocity`))))))

(fn `SetYRotation`
  (params (Target :type "SceneComponent Object Reference"))
  ;[1 1 1] Set "Y" rotation velocity
  (set `self.Y_Velocity` (`KismetMathLibrary.Abs` (.yaw (`KismetMathLibrary.RInterpTo` (`SceneComponent.RelativeRotation` (`self.Mesh`)) (`SceneComponent.RelativeRotation` Target) (`self.DeltaSec`) 2.0)))))