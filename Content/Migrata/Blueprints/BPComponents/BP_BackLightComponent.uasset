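; BP_BackLightComponent is a destructible vehicle back light with glass, plastic and mesh parts.
; ToggleLights applies a red material to two light meshes, with no path back.
; Any hit on the light mesh makes all three meshes simulate physics and block the Vehicle channel.
; A separate impulse-based damage function, uncalled here, breaks a part when one hit exceeds its HP, storing HP only then.
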(event `ToggleLights`
  (`PrimitiveComponent.SetMaterial` (`self.ST_Light_B`) 1 "/Game/Migrata/Materials/MainMat/MI_Lights/MI_RedLIght.MI_RedLIght")
  (`PrimitiveComponent.SetMaterial` (`self.ST_Light_B_Plastic`) 1 "/Game/Migrata/Materials/MainMat/MI_Lights/MI_RedLIght.MI_RedLIght"))

(event `self.ST_Light_B.OnComponentHit`
  (params (HitComponent :type "PrimitiveComponent Object Reference") (OtherActor :type "Actor Object Reference") (OtherComp :type "PrimitiveComponent Object Reference") (NormalImpulse :type "Vector Structure") (Hit :type "HitResult Structure (by ref)"))
  (`PrimitiveComponent.SetSimulatePhysics` (`self.ST_Light_B_Plastic`) true)
  (`PrimitiveComponent.SetSimulatePhysics` (`self.StaticMesh`) true)
  (`PrimitiveComponent.SetSimulatePhysics` (`self.ST_Light_B`) true)
  (`PrimitiveComponent.SetCollisionResponseToChannel` (`self.ST_Light_B`) "ECC_Vehicle" "ECR_Block")
  (`PrimitiveComponent.SetCollisionResponseToChannel` (`self.StaticMesh`) "ECC_Vehicle" "ECR_Block")
  (`PrimitiveComponent.SetCollisionResponseToChannel` (`self.ST_Light_B_Plastic`) "ECC_Vehicle" "ECR_Block"))

(fn `Destructable Parts Simple`
  (params (Impulse :type "Vector Structure") (damagedPartInfo1 :type "/Game/Migrata/Blueprints/Struct/Part_Struct Structure (by ref)") (DestructablePar :type "PrimitiveComponent Object Reference"))
  (bind _destructablepar (`local.DestructablePar`))
  (bind ((`Name_28_4809519E479B4BE740F4BAB2C5B99A76` _name) (`MartDamagedMesh_25_7458C1AD4F5C10D753638B93A251DB13` _martdamagedmesh) (`HP_12_FC4B2F15485B81F0C0FDCF89F71E6102` _hp) (`PartDamaged_17_77E7AD59459221392C43448ACB01BE4D` _partdamaged) (`PartOpened_13_3293DDB54951A737FCCC96BA2644690C` _partopened)) (break `/Game/Migrata/Blueprints/Struct/Part_Struct` (`local.damagedPartInfo1`)))
  (bind _returnvalue (/ (`KismetMathLibrary.Abs` (+ (.x Impulse) (.y Impulse) (.z Impulse))) 10000.0))
  (bind _returnvalue_2 (- _hp _returnvalue))
  (`|ExecutionSequence`
    (:`then_0`
      ;[1 1 1] Do Sometging if impulse more than N
      (set `self.DamagedPartLocal` damagedPartInfo1)
      (if (> _returnvalue 1.0)
        ;[1 1 1] DOOnceOpeningPart
        (if (not _partopened)
          ;[1 1 1] ComponentHP
          (if (< _returnvalue_2 0.0)
            ;[1 1 1] Part Simulating if HP is <0
            (setmembers `/Game/Migrata/Blueprints/Struct/Part_Struct` :`StructRef` (`self.DamagedPartLocal`) :`HP` _returnvalue_2 :`PartBroken` true)
            (`PrimitiveComponent.SetSimulatePhysics` _destructablepar true)
            ;[1 1 1] DisableHitEentAndReturnLastCarVelocity
            (`PrimitiveComponent.SetNotifyRigidBodyCollision` _destructablepar false)))))
    (:`then_1`
      (`|VariableSetRef` damagedPartInfo1 (`self.DamagedPartLocal`)))))

(fn `UserConstructionScript`)