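; Drivable car pawn with impact-based part damage, first- and third-person cameras, and an animated steering wheel.
; Input feeds the vehicle movement component and a camera component that handles zoom, look, side/rear views and switching.
; Component hits pass impulses to two struct-driven functions: hinged panels swap to damaged meshes, lose HP, then swing on physics constraints.
; Simple parts detach when one hit exceeds their HP; light toggle and mirror hits are empty.
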(event `Key|L`
  (params (Key :type "Key Structure"))
  (:`Pressed`
    (`self.ToggleLight`)))

(event `ToggleLight`)

(event `InputAxisKey|MouseWheelAxis`
  (params (AxisValue :type "Float (single-precision)"))
  ;[0 1 0.1918] CameraMovement
  (`/Game/Migrata/DynamicCarCameraSystem/Blueprints/BP_CameraCompSkeletalMesh.CameraZoom` (`self.CameraCompSkeletalMesh`) AxisValue))

(event `InputAxis|MouseLook`
  (params (AxisValue :type "Float (single-precision)"))
  ;[0 1 0.1918] Mouse
  (`/Game/Migrata/DynamicCarCameraSystem/Blueprints/BP_CameraCompSkeletalMesh.MouseActivating` (`self.CameraCompSkeletalMesh`) (`self.GetInputAxisValue`) (`self.GetInputAxisValue`) (`KismetMathLibrary.InRange_FloatFloat` AxisValue -0.2 0.2)))

(event `self.ReceiveTick`
  (params (DeltaSeconds :type "Float (single-precision)"))
  (bind _returnvalue (`self.GetInputAxisValue`))
  (bind _steering_wheel (`self.Steering_Wheel`))
  (`|ExecutionSequence`
    (:`then_0`
      ;[1 1 1] BackLight
      (if (`self.Lights_Front_ON`)
        (if (== (`WheeledVehicleMovementComponent.GetCurrentGear` (`self.VehicleMovement`)) -1)
          (`PrimitiveComponent.SetMaterial` (`self.Headlight_B_L`) 3 null)
          (goto _label :!via `Reset`)
          (else
            (`/Engine/EditorBlueprintResources/StandardMacros.DoOnce` false :!label _label
              (:`Completed`
                (`PrimitiveComponent.SetMaterial` null 3 null)
                (`PrimitiveComponent.SetMaterial` (`self.Headlight_B_L`) 3 null)))))))
    (:`then_1`
      ;[1 1 1] SteeringWheelRotation
      (if (== _returnvalue 0.0)
        (bind _output_get (set `self.WheelRotation` (* (`self.WheelRotation`) 0.8)))
        (`SceneComponent.K2_SetRelativeRotation` _steering_wheel (`KismetMathLibrary.MakeRotator` _output_get -30.0) false false)
        (else
          (bind _output_get_2 (set `self.WheelRotation` (`KismetMathLibrary.FClamp` (+ (* _returnvalue 2.0) (`self.WheelRotation`)) -100.0 100.0)))
          (`SceneComponent.K2_SetRelativeRotation` _steering_wheel (`KismetMathLibrary.MakeRotator` _output_get_2 -30.0) false false))))
    (:`then_2`
      (bind _returnvalue_2 (`PrimitiveComponent.GetPhysicsLinearVelocity` (`self.Mesh`) "None"))
      (set `self.CarVelocity` _returnvalue_2))))

(event `Key|Q`
  (params (Key :type "Key Structure"))
  (bind _cameracompskeletalmesh (`self.CameraCompSkeletalMesh`))
  ;[0 1 0.1918] CameraMovement
  (:`Pressed`
    (`/Game/Migrata/DynamicCarCameraSystem/Blueprints/BP_CameraCompSkeletalMesh.ButtonPressed` _cameracompskeletalmesh 60.0))
  (:`Released`
    (`/Game/Migrata/DynamicCarCameraSystem/Blueprints/BP_CameraCompSkeletalMesh.ButtonReleased` _cameracompskeletalmesh)))

(event `Key|E`
  (params (Key :type "Key Structure"))
  (bind _cameracompskeletalmesh (`self.CameraCompSkeletalMesh`))
  ;[0 1 0.1918] CameraMovement
  (:`Pressed`
    (`/Game/Migrata/DynamicCarCameraSystem/Blueprints/BP_CameraCompSkeletalMesh.ButtonPressed` _cameracompskeletalmesh -60.0))
  (:`Released`
    (`/Game/Migrata/DynamicCarCameraSystem/Blueprints/BP_CameraCompSkeletalMesh.ButtonReleased` _cameracompskeletalmesh)))

(event `self.ReceiveBeginPlay`
  (`self.SetCameraComp`))

(event `Key|MiddleMouseButton`
  (params (Key :type "Key Structure"))
  (bind _cameracompskeletalmesh (`self.CameraCompSkeletalMesh`))
  ;[0 1 0.1918] CameraMovement
  (:`Pressed`
    (`/Game/Migrata/DynamicCarCameraSystem/Blueprints/BP_CameraCompSkeletalMesh.ButtonPressed` _cameracompskeletalmesh 180.0))
  (:`Released`
    (`/Game/Migrata/DynamicCarCameraSystem/Blueprints/BP_CameraCompSkeletalMesh.ButtonReleased` _cameracompskeletalmesh)))

(event `Key|V`
  (params (Key :type "Key Structure"))
  ;[0 1 0.2621] ChangeCamera
  (:`Pressed`
    (`/Game/Migrata/DynamicCarCameraSystem/Blueprints/BP_CameraCompSkeletalMesh.ChangeCamera` (`self.CameraCompSkeletalMesh`))))

(event `self.Hood_F.OnComponentHit`
  (params (HitComponent :type "PrimitiveComponent Object Reference") (OtherActor :type "Actor Object Reference") (OtherComp :type "PrimitiveComponent Object Reference") (NormalImpulse :type "Vector Structure") (Hit :type "HitResult Structure (by ref)"))
  ;[1 1 1] HoodDestruction
  (`self.Destructble Parts With Constraint` NormalImpulse (`self.Hood_F`) (`self.Body_B`) (`self.HoodConstraint`) (`self.Hood_F_Struct`))
  (`StaticMeshComponent.SetStaticMesh` (`self.Body_F`) "/Game/Migrata/Meshes/BodyDamaged/ST_Body_F_Damaged.ST_Body_F_Damaged"))

(event `self.Headlight_F_R.OnComponentHit`
  (params (HitComponent :type "PrimitiveComponent Object Reference") (OtherActor :type "Actor Object Reference") (OtherComp :type "PrimitiveComponent Object Reference") (NormalImpulse :type "Vector Structure") (Hit :type "HitResult Structure (by ref)"))
  ;[1 1 1] LightDestructoion
  (`self.Destructible Parts Simple` NormalImpulse (`|GetArrayItem` (`self.SiimplePartStruct`) 14) HitComponent)
  (`KismetSystemLibrary.PrintString` "Hello"))

(event `self.ST_ExtPart_02_FL.OnComponentHit`
  (params (HitComponent :type "PrimitiveComponent Object Reference") (OtherActor :type "Actor Object Reference") (OtherComp :type "PrimitiveComponent Object Reference") (NormalImpulse :type "Vector Structure") (Hit :type "HitResult Structure (by ref)"))
  ;[1 1 1] WingsDestruction
  (`self.Destructible Parts Simple` NormalImpulse (`|GetArrayItem` (`self.SiimplePartStruct`) 6) HitComponent))

(event `self.Hood_B.OnComponentHit`
  (params (HitComponent :type "PrimitiveComponent Object Reference") (OtherActor :type "Actor Object Reference") (OtherComp :type "PrimitiveComponent Object Reference") (NormalImpulse :type "Vector Structure") (Hit :type "HitResult Structure (by ref)"))
  ;[1 1 1] HoodDestruction
  (`self.Destructble Parts With Constraint` NormalImpulse (`self.Hood_B`) (`self.Body_B`) (`self.Hood_B_Constraint`) (`self.Hood_B_Struct`)))

(event `self.Headlight_F_L.OnComponentHit`
  (params (HitComponent :type "PrimitiveComponent Object Reference") (OtherActor :type "Actor Object Reference") (OtherComp :type "PrimitiveComponent Object Reference") (NormalImpulse :type "Vector Structure") (Hit :type "HitResult Structure (by ref)"))
  ;[1 1 1] LightDestructoion
  (`self.Destructible Parts Simple` NormalImpulse (`|GetArrayItem` (`self.SiimplePartStruct`) 15) HitComponent))

(event `self.ST_ExtPart_03_BL.OnComponentHit`
  (params (HitComponent :type "PrimitiveComponent Object Reference") (OtherActor :type "Actor Object Reference") (OtherComp :type "PrimitiveComponent Object Reference") (NormalImpulse :type "Vector Structure") (Hit :type "HitResult Structure (by ref)"))
  ;[1 1 1] WingsDestruction
  (`self.Destructible Parts Simple` NormalImpulse (`|GetArrayItem` (`self.SiimplePartStruct`) 9) HitComponent))

(event `self.Si_ExtPart_04.OnComponentHit`
  (params (HitComponent :type "PrimitiveComponent Object Reference") (OtherActor :type "Actor Object Reference") (OtherComp :type "PrimitiveComponent Object Reference") (NormalImpulse :type "Vector Structure") (Hit :type "HitResult Structure (by ref)"))
  ;[1 1 1] FrontParts
  (`self.Destructible Parts Simple` NormalImpulse (`|GetArrayItem` (`self.SiimplePartStruct`) 1) HitComponent))

(event `self.ST_ExtPart_02_FL1.OnComponentHit`
  (params (HitComponent :type "PrimitiveComponent Object Reference") (OtherActor :type "Actor Object Reference") (OtherComp :type "PrimitiveComponent Object Reference") (NormalImpulse :type "Vector Structure") (Hit :type "HitResult Structure (by ref)"))
  ;[1 1 1] WingsDestruction
  (`self.Destructible Parts Simple` NormalImpulse (`|GetArrayItem` (`self.SiimplePartStruct`) 6) HitComponent))

(event `self.Fender_L.OnComponentHit`
  (params (HitComponent :type "PrimitiveComponent Object Reference") (OtherActor :type "Actor Object Reference") (OtherComp :type "PrimitiveComponent Object Reference") (NormalImpulse :type "Vector Structure") (Hit :type "HitResult Structure (by ref)"))
  ;[1 1 1] FenderDestruction
  (`self.Destructble Parts With Constraint` NormalImpulse (`self.Fender_L`) (`self.Body_B`) (`self.Fender_L_COnstraint`) (`self.Fender_L_Struct`)))

(event `self.Si_ExtPart_06.OnComponentHit`
  (params (HitComponent :type "PrimitiveComponent Object Reference") (OtherActor :type "Actor Object Reference") (OtherComp :type "PrimitiveComponent Object Reference") (NormalImpulse :type "Vector Structure") (Hit :type "HitResult Structure (by ref)"))
  ;[1 1 1] FrontParts
  (`self.Destructible Parts Simple` NormalImpulse (`|GetArrayItem` (`self.SiimplePartStruct`)) HitComponent))

(event `self.ST_ExtPart_01_L.OnComponentHit`
  (params (HitComponent :type "PrimitiveComponent Object Reference") (OtherActor :type "Actor Object Reference") (OtherComp :type "PrimitiveComponent Object Reference") (NormalImpulse :type "Vector Structure") (Hit :type "HitResult Structure (by ref)"))
  ;[1 1 1] SkirtDestruction
  (`self.Destructible Parts Simple` NormalImpulse (`|GetArrayItem` (`self.SiimplePartStruct`) 16) HitComponent))

(event `self.ST_ExtPart_03_BL1.OnComponentHit`
  (params (HitComponent :type "PrimitiveComponent Object Reference") (OtherActor :type "Actor Object Reference") (OtherComp :type "PrimitiveComponent Object Reference") (NormalImpulse :type "Vector Structure") (Hit :type "HitResult Structure (by ref)"))
  ;[1 1 1] WingsDestruction
  (`self.Destructible Parts Simple` NormalImpulse (`|GetArrayItem` (`self.SiimplePartStruct`) 8) HitComponent))

(event `self.ST_ExtPart_011.OnComponentHit`
  (params (HitComponent :type "PrimitiveComponent Object Reference") (OtherActor :type "Actor Object Reference") (OtherComp :type "PrimitiveComponent Object Reference") (NormalImpulse :type "Vector Structure") (Hit :type "HitResult Structure (by ref)"))
  ;[1 1 1] FrontParts
  (`self.Destructible Parts Simple` NormalImpulse (`|GetArrayItem` (`self.SiimplePartStruct`) 2) HitComponent))

(event `self.Fender_R.OnComponentHit`
  (params (HitComponent :type "PrimitiveComponent Object Reference") (OtherActor :type "Actor Object Reference") (OtherComp :type "PrimitiveComponent Object Reference") (NormalImpulse :type "Vector Structure") (Hit :type "HitResult Structure (by ref)"))
  ;[1 1 1] FenderDestruction
  (`self.Destructble Parts With Constraint` NormalImpulse (`self.Fender_R`) (`self.Body_B`) (`self.Fender_FR_Constraint`) (`self.Fender_R_Struct`)))

(event `self.ST_ExtPart_01_R.OnComponentHit`
  (params (HitComponent :type "PrimitiveComponent Object Reference") (OtherActor :type "Actor Object Reference") (OtherComp :type "PrimitiveComponent Object Reference") (NormalImpulse :type "Vector Structure") (Hit :type "HitResult Structure (by ref)"))
  ;[1 1 1] SkirtDestruction
  (`self.Destructible Parts Simple` NormalImpulse (`|GetArrayItem` (`self.SiimplePartStruct`) 17) HitComponent))

(event `self.ST_ExtPart_05.OnComponentHit`
  (params (HitComponent :type "PrimitiveComponent Object Reference") (OtherActor :type "Actor Object Reference") (OtherComp :type "PrimitiveComponent Object Reference") (NormalImpulse :type "Vector Structure") (Hit :type "HitResult Structure (by ref)"))
  ;[1 1 1] FrontParts
  (`self.Destructible Parts Simple` NormalImpulse (`|GetArrayItem` (`self.SiimplePartStruct`) 3) HitComponent))

(event `self.ST_ExtPart_16.OnComponentHit`
  (params (HitComponent :type "PrimitiveComponent Object Reference") (OtherActor :type "Actor Object Reference") (OtherComp :type "PrimitiveComponent Object Reference") (NormalImpulse :type "Vector Structure") (Hit :type "HitResult Structure (by ref)"))
  (`self.Destructible Parts Simple` NormalImpulse (`|GetArrayItem` (`self.SiimplePartStruct`) 10) HitComponent))

(event `self.w.OnComponentHit`
  (params (HitComponent :type "PrimitiveComponent Object Reference") (OtherActor :type "Actor Object Reference") (OtherComp :type "PrimitiveComponent Object Reference") (NormalImpulse :type "Vector Structure") (Hit :type "HitResult Structure (by ref)"))
  (`self.Destructible Parts Simple` NormalImpulse (`|GetArrayItem` (`self.SiimplePartStruct`) 17) HitComponent))

(event `self.Prot_F.OnComponentHit`
  (params (HitComponent :type "PrimitiveComponent Object Reference") (OtherActor :type "Actor Object Reference") (OtherComp :type "PrimitiveComponent Object Reference") (NormalImpulse :type "Vector Structure") (Hit :type "HitResult Structure (by ref)"))
  ;[1 1 1] FrontParts
  (`self.Destructible Parts Simple` NormalImpulse (`|GetArrayItem` (`self.SiimplePartStruct`) 4) HitComponent))

(event `self.Bumper_B.OnComponentHit`
  (params (HitComponent :type "PrimitiveComponent Object Reference") (OtherActor :type "Actor Object Reference") (OtherComp :type "PrimitiveComponent Object Reference") (NormalImpulse :type "Vector Structure") (Hit :type "HitResult Structure (by ref)"))
  ;[1 1 1] BumperDestruction
  (`self.Destructble Parts With Constraint` NormalImpulse (`self.Bumper_B`) (`self.Body_B`) (`self.Bumper_B_Constraint`) (`self.Bumper_B_Struct`)))

(event `self.ST_ExtPart_17.OnComponentHit`
  (params (HitComponent :type "PrimitiveComponent Object Reference") (OtherActor :type "Actor Object Reference") (OtherComp :type "PrimitiveComponent Object Reference") (NormalImpulse :type "Vector Structure") (Hit :type "HitResult Structure (by ref)"))
  (`self.Destructible Parts Simple` NormalImpulse (`|GetArrayItem` (`self.SiimplePartStruct`) 11) HitComponent))

(event `self.ST_ExtPart_07.OnComponentHit`
  (params (HitComponent :type "PrimitiveComponent Object Reference") (OtherActor :type "Actor Object Reference") (OtherComp :type "PrimitiveComponent Object Reference") (NormalImpulse :type "Vector Structure") (Hit :type "HitResult Structure (by ref)"))
  (`self.Destructible Parts Simple` NormalImpulse (`|GetArrayItem` (`self.SiimplePartStruct`) 17) HitComponent))

(event `self.Exhaust.OnComponentHit`
  (params (HitComponent :type "PrimitiveComponent Object Reference") (OtherActor :type "Actor Object Reference") (OtherComp :type "PrimitiveComponent Object Reference") (NormalImpulse :type "Vector Structure") (Hit :type "HitResult Structure (by ref)"))
  ;[1 1 1] FrontParts
  (`self.Destructible Parts Simple` NormalImpulse (`|GetArrayItem` (`self.SiimplePartStruct`) 3) HitComponent))

(event `self.NumbLow1.OnComponentHit`
  (params (HitComponent :type "PrimitiveComponent Object Reference") (OtherActor :type "Actor Object Reference") (OtherComp :type "PrimitiveComponent Object Reference") (NormalImpulse :type "Vector Structure") (Hit :type "HitResult Structure (by ref)"))
  (`self.Destructible Parts Simple` NormalImpulse (`|GetArrayItem` (`self.SiimplePartStruct`) 20) HitComponent))

(event `self.Door_F_R.OnComponentHit`
  (params (HitComponent :type "PrimitiveComponent Object Reference") (OtherActor :type "Actor Object Reference") (OtherComp :type "PrimitiveComponent Object Reference") (NormalImpulse :type "Vector Structure") (Hit :type "HitResult Structure (by ref)"))
  (bind _st_extpart_010 (`self.ST_ExtPart_010`))
  ;[1 1 1] DoorsDestruction
  (`self.Destructble Parts With Constraint` NormalImpulse (`self.Door_F_R`) (`self.Body_B`) (`self.Door_FR_Constraint`) (`self.Door_FR_Struct`))
  (`PrimitiveComponent.SetSimulatePhysics` _st_extpart_010 true)
  (`PrimitiveComponent.SetCollisionProfileName` _st_extpart_010 "BlockAll" true))

(event `self.Spoiler_0.OnComponentHit`
  (params (HitComponent :type "PrimitiveComponent Object Reference") (OtherActor :type "Actor Object Reference") (OtherComp :type "PrimitiveComponent Object Reference") (NormalImpulse :type "Vector Structure") (Hit :type "HitResult Structure (by ref)"))
  ;[1 1 1] FrontParts
  (`self.Destructible Parts Simple` NormalImpulse (`|GetArrayItem` (`self.SiimplePartStruct`) 5) HitComponent))

(event `self.Door_B_R.OnComponentHit`
  (params (HitComponent :type "PrimitiveComponent Object Reference") (OtherActor :type "Actor Object Reference") (OtherComp :type "PrimitiveComponent Object Reference") (NormalImpulse :type "Vector Structure") (Hit :type "HitResult Structure (by ref)"))
  (bind _st_extpart_13 (`self.ST_ExtPart_13`))
  ;[1 1 1] DoorsDestruction
  (`self.Destructble Parts With Constraint` NormalImpulse (`self.Door_B_R`) (`self.Body_B`) (`self.Door_BR_Constraint`) (`self.Door_BR_Struct`))
  (`PrimitiveComponent.SetSimulatePhysics` _st_extpart_13 true)
  (`PrimitiveComponent.SetCollisionProfileName` _st_extpart_13 "BlockAll" true))

(event `self.Mirror_L.OnComponentHit`
  (params (HitComponent :type "PrimitiveComponent Object Reference") (OtherActor :type "Actor Object Reference") (OtherComp :type "PrimitiveComponent Object Reference") (NormalImpulse :type "Vector Structure") (Hit :type "HitResult Structure (by ref)"))
  ;[1 1 1] Mirrors
)

(event `self.Mirror_R.OnComponentHit`
  (params (HitComponent :type "PrimitiveComponent Object Reference") (OtherActor :type "Actor Object Reference") (OtherComp :type "PrimitiveComponent Object Reference") (NormalImpulse :type "Vector Structure") (Hit :type "HitResult Structure (by ref)"))
  ;[1 1 1] Mirrors
)

(event `self.Door_B_L.OnComponentHit`
  (params (HitComponent :type "PrimitiveComponent Object Reference") (OtherActor :type "Actor Object Reference") (OtherComp :type "PrimitiveComponent Object Reference") (NormalImpulse :type "Vector Structure") (Hit :type "HitResult Structure (by ref)"))
  (bind _st_extpart_10 (`self.ST_ExtPart_10`))
  ;[1 1 1] DoorsDestruction
  (`self.Destructble Parts With Constraint` NormalImpulse (`self.Door_B_L`) (`self.Body_B`) (`self.Door_BL_Constraint`) (`self.Door_BL_Struct`))
  (`PrimitiveComponent.SetSimulatePhysics` _st_extpart_10 true)
  (`PrimitiveComponent.SetCollisionProfileName` _st_extpart_10 "BlockAll" true))

(event `self.Door_FL.OnComponentHit`
  (params (HitComponent :type "PrimitiveComponent Object Reference") (OtherActor :type "Actor Object Reference") (OtherComp :type "PrimitiveComponent Object Reference") (NormalImpulse :type "Vector Structure") (Hit :type "HitResult Structure (by ref)"))
  (bind _st_extpart_09 (`self.ST_ExtPart_09`))
  ;[1 1 1] DoorsDestruction
  (`self.Destructble Parts With Constraint` NormalImpulse (`self.Door_FL`) (`self.Body_B`) (`self.Door_FL_COnstraint`) (`self.Door_FL_Struct`))
  (`PrimitiveComponent.SetSimulatePhysics` _st_extpart_09 true)
  (`PrimitiveComponent.SetCollisionProfileName` _st_extpart_09 "BlockAll" true))

(event `Key|Tab`
  (params (Key :type "Key Structure"))
  (:`Pressed`
    (`KismetSystemLibrary.ExecuteConsoleCommand` "PXVIS COLLISION" (`GameplayStatics.GetPlayerController` 0))))

(event `InputAxis|Turn`
  (params (AxisValue :type "Float (single-precision)"))
  ;[1 1 1] Wehicle Movement
  (`WheeledVehicleMovementComponent.SetSteeringInput` (`self.VehicleMovement`) AxisValue))

(event `InputAxis|Acceleration`
  (params (AxisValue :type "Float (single-precision)"))
  ;[1 1 1] Wehicle Movement
  (`WheeledVehicleMovementComponent.SetThrottleInput` (`self.VehicleMovement`) AxisValue))

(event `InputAction|Handbrake`
  (params (Key :type "Key Structure"))
  (bind _vehiclemovement (`self.VehicleMovement`))
  ;[1 1 1] Wehicle Movement
  (:`Pressed`
    (`WheeledVehicleMovementComponent.SetHandbrakeInput` _vehiclemovement true))
  (:`Released`
    (`WheeledVehicleMovementComponent.SetHandbrakeInput` _vehiclemovement false)))

(fn `Destructble Parts With Constraint`
  (params (Impulse :type "Vector Structure") (DestructablePart :type "StaticMeshComponent Object Reference") (ParentComp1 :type "StaticMeshComponent Object Reference") (Constraint1 :type "PhysicsConstraintComponent Object Reference") (damagedPartInfo1 :type "/Game/Migrata/Blueprints/Struct/Part_Struct Structure (by ref)"))
  (locals (DamagedPartLocal :type "/Game/Migrata/Blueprints/Struct/Part_Struct Structure"))
  (bind _destructablepart (`local.DestructablePart`))
  (bind ((`Name_28_4809519E479B4BE740F4BAB2C5B99A76` _name) (`MartDamagedMesh_25_7458C1AD4F5C10D753638B93A251DB13` _martdamagedmesh) (`HP_12_FC4B2F15485B81F0C0FDCF89F71E6102` _hp) (`PartDamaged_17_77E7AD59459221392C43448ACB01BE4D` _partdamaged) (`PartOpened_13_3293DDB54951A737FCCC96BA2644690C` _partopened)) (break `/Game/Migrata/Blueprints/Struct/Part_Struct` (`local.damagedPartInfo1`)))
  (bind _returnvalue (/ (`KismetMathLibrary.Abs` (+ (.x Impulse) (.y Impulse) (.z Impulse))) 10000.0))
  (bind _returnvalue_2 (- _hp _returnvalue))
  (`|ExecutionSequence`
    (:`then_0`
      ;[1 1 1] Do Sometging if impulse more than N
      (set `local.DamagedPartLocal` damagedPartInfo1)
      (if (> _returnvalue 1.0)
        (`|ExecutionSequence`
          (:`then_0`
            ;[1 1 1] DoOncePartDamageModel
            (if (not _partdamaged)
              ;[1 1 1] SetDamagedComponent
              (`StaticMeshComponent.SetStaticMesh` (`local.DestructablePart`) _martdamagedmesh)
              (setmembers `/Game/Migrata/Blueprints/Struct/Part_Struct` :`StructRef` (`local.DamagedPartLocal`) :`PartDamaged` true)))
          (:`then_1`
            ;[1 1 1] DOOnceOpeningPart
            (if (not _partopened)
              ;[1 1 1] ComponentHP
              (setmembers `/Game/Migrata/Blueprints/Struct/Part_Struct` :`StructRef` (`local.DamagedPartLocal`) :`HP` _returnvalue_2)
              (if (< _returnvalue_2 0.0)
                ;[1 1 1] Part opening if HP is <0
                (`PrimitiveComponent.SetSimulatePhysics` _destructablepart true)
                (`PhysicsConstraintComponent.SetConstrainedComponents` (`local.Constraint1`) (`local.ParentComp1`) "None" _destructablepart "None")
                (setmembers `/Game/Migrata/Blueprints/Struct/Part_Struct` :`StructRef` (`local.DamagedPartLocal`) :`PartOpened` true)))))))
    (:`then_1`
      (`|VariableSetRef` damagedPartInfo1 (`local.DamagedPartLocal`)))))

(fn `Destructible Parts Simple`
  (params (Impulse :type "Vector Structure") (damagedPartInfo1 :type "/Game/Migrata/Blueprints/Struct/Part_Struct Structure (by ref)") (DestructiblePar :type "PrimitiveComponent Object Reference"))
  (locals (DamagedPartLocal :type "/Game/Migrata/Blueprints/Struct/Part_Struct Structure"))
  (bind _destructiblepar (`local.DestructiblePar`))
  (bind ((`Name_28_4809519E479B4BE740F4BAB2C5B99A76` _name) (`MartDamagedMesh_25_7458C1AD4F5C10D753638B93A251DB13` _martdamagedmesh) (`HP_12_FC4B2F15485B81F0C0FDCF89F71E6102` _hp) (`PartDamaged_17_77E7AD59459221392C43448ACB01BE4D` _partdamaged) (`PartOpened_13_3293DDB54951A737FCCC96BA2644690C` _partopened)) (break `/Game/Migrata/Blueprints/Struct/Part_Struct` (`local.damagedPartInfo1`)))
  (bind _returnvalue (/ (`KismetMathLibrary.Abs` (+ (.x Impulse) (.y Impulse) (.z Impulse))) 10000.0))
  (bind _returnvalue_2 (- _hp _returnvalue))
  (`|ExecutionSequence`
    (:`then_0`
      ;[1 1 1] Do Sometging if impulse more than N
      (set `local.DamagedPartLocal` damagedPartInfo1)
      (if (> _returnvalue 1.0)
        ;[1 1 1] DOOnceOpeningPart
        (if (not _partopened)
          ;[1 1 1] ComponentHP
          (if (< _returnvalue_2 0.0)
            ;[1 1 1] Part Simulating if HP is <0
            (setmembers `/Game/Migrata/Blueprints/Struct/Part_Struct` :`StructRef` (`local.DamagedPartLocal`) :`HP` _returnvalue_2 :`PartBroken` true)
            (`PrimitiveComponent.SetSimulatePhysics` _destructiblepar true)
            ;[1 1 1] DisableHitEentAndReturnLastCarVelocity
            (`PrimitiveComponent.SetNotifyRigidBodyCollision` _destructiblepar false)))))
    (:`then_1`
      (`|VariableSetRef` damagedPartInfo1 (`local.DamagedPartLocal`)))))

(fn `SetCameraComp`
  (bind _cameracompskeletalmesh (`self.CameraCompSkeletalMesh`))
  (set `/Game/Migrata/DynamicCarCameraSystem/Blueprints/BP_CameraCompSkeletalMesh.CameraID` 0 _cameracompskeletalmesh)
  (set `/Game/Migrata/DynamicCarCameraSystem/Blueprints/BP_CameraCompSkeletalMesh.Mesh` (`self.Mesh`) _cameracompskeletalmesh)
  (set `/Game/Migrata/DynamicCarCameraSystem/Blueprints/BP_CameraCompSkeletalMesh.3rdcamera` (`self.3RdCamera1`) _cameracompskeletalmesh)
  (set `/Game/Migrata/DynamicCarCameraSystem/Blueprints/BP_CameraCompSkeletalMesh.1stCamera` (`self.1StCamera`) _cameracompskeletalmesh)
  (set `/Game/Migrata/DynamicCarCameraSystem/Blueprints/BP_CameraCompSkeletalMesh.SpringArm3rd` (`self.3RdSpringArm1`) _cameracompskeletalmesh)
  (set `/Game/Migrata/DynamicCarCameraSystem/Blueprints/BP_CameraCompSkeletalMesh.SpringArm1st` (`self.1StSpringArm`) _cameracompskeletalmesh)
  (set `/Game/Migrata/DynamicCarCameraSystem/Blueprints/BP_CameraCompSkeletalMesh.SceneComponent1St` (`self.1StcameraComp`) _cameracompskeletalmesh)
  (set `/Game/Migrata/DynamicCarCameraSystem/Blueprints/BP_CameraCompSkeletalMesh.SceneComponent3rd` (`self.3RdCameraComp`) _cameracompskeletalmesh))

(fn `UserConstructionScript`)