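; Player controller that shows a car selection screen at game start and hands control over according to the choice.
; BeginPlay adds the WBP_Game_Mode widget to the viewport and binds its ChooseCar event.
; On selection, it collapses the widget, hides the cursor and switches to game-only input.
; Each option, Agron or Agron Susp, runs its own GetAllActorsOfClass lookup and Possess call.
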(event `self.ReceiveBeginPlay`
  (bind _returnvalue (`|CreateWidget` "/Game/Migrata/Blueprints/WBP_Game_Mode.WBP_Game_Mode_C"))
  (`UserWidget.AddToViewport` _returnvalue 0)
  (add `/Game/Migrata/Blueprints/WBP_Game_Mode.ChooseCar` _returnvalue (delegate `ChoooseCar`)))

(event `ChoooseCar`
  (params (Agron :type Name))
  (bind _returnvalue (`GameplayStatics.GetPlayerController` 0))
  ;[1 1 1] ChooseCar
  (`Widget.SetVisibility` (stale `self.ReceiveBeginPlay` _returnvalue) "Collapsed")
  (set `PlayerController.bShowMouseCursor` false _returnvalue)
  (`WidgetBlueprintLibrary.SetInputMode_GameOnly` _returnvalue)
  (switch `name` Agron
    (:`Agron`
      (bind _outactors (`GameplayStatics.GetAllActorsOfClass` null))
      (`self.Possess` null))
    (:`AgronSusp`
      (bind _outactors_2 (`GameplayStatics.GetAllActorsOfClass` null))
      (`self.Possess` null))))

(fn `UserConstructionScript`)